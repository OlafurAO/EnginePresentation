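; A behavior tree task that finds the current patrol point for an AI-TEST pawn.
; It reads the path index from the blackboard, converts that PatrolPath point from the path actor's local space to world space, and writes it to the path vector key.
; It finishes only on success; a failed cast or missing path leaves the task without a finish call.
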(event EventReceiveExecuteAI
  (params (OwnerController :type AI%20Controller%20Object%20Reference) (ControlledPawn :type Pawn%20Object%20Reference))
  (bind _asai_test (Utilities|Casting|CastToAI-TEST ControlledPawn))
  (bind _patrolpath (Variables|/Game/Blueprints/AI/AI-TEST.AI-TEST_C|GetPatrolPath _asai_test)
    (:then
      (AI|BehaviorTree|SetBlackboardValueasVector (Variables|Default|GetBB_Path_Vector) (Math|Transform|TransformLocation (Transformation|GetActorTransform _patrolpath) (Utilities|Array|Get(acopy) (Variables|/Game/Blueprints/AI/PatrolPath.PatrolPath_C|GetPathPoints _patrolpath) (Class|BTFunctionLibrary|GetBlackboardValueasInt (Variables|Default|GetBB_Path_Index)))))
      (AI|BehaviorTree|FinishExecute true))
    (:else)))