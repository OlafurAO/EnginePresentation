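; Test AI character Blueprint, judging by its name, with aim/sprint movement speeds and a Fullyauto gun-fire function.
; UpdateMovementSpeed sets walk speed from the aiming and sprinting flags, with aiming taking priority.
; Fullyauto plays a sound and spawns a KA47 bullet at the Muzzle transform.
; Its muzzle flash, HUD and ammo decrement, and low-ammo timer stop are disconnected and never run.
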(fn ConstructionScript)

(fn UpdateMovementSpeed
  (bind _charactermovement (Variables|Character|GetCharacterMovement))
  (if (Variables|Default|GetIsAiming)
    (Variables|/Script/Engine.CharacterMovementComponent|SetMaxWalkSpeed _charactermovement 2.5e+02)
    (elif (Variables|Default|GetIsSprinting)
      (Variables|/Script/Engine.CharacterMovementComponent|SetMaxWalkSpeed _charactermovement 7.5e+02)
      (else
        (Variables|/Script/Engine.CharacterMovementComponent|SetMaxWalkSpeed _charactermovement 5e+02)))))

(fn Fullyauto
  (Audio|PlaySoundatLocation 0 "0, 0, 0" "0, 0, 0" 1.0 1.0 0.0 0 0 0)
  (Game|SpawnActorfromClass "/Game/Blueprints/BP_KA47_Bullet.BP_KA47_Bullet_C" (Transformation|GetWorldTransform (Variables|Default|GetMuzzle)) "Undefined" 0 0))