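; AI controller that starts the AItreetest behavior tree for an AI-TEST pawn.
; On BeginPlay it seeds the blackboard with looping and wait time from the pawn's patrol path, plus an initial direction.
; AI Perception updates set the visablePlayer key to whether a BP_Character is currently sensed.
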(event OnTargetPerceptionUpdated(AIPerception)
  (params (Actor :type Actor%20Object%20Reference) (Stimulus :type AI%20Stimulus%20Structure))
  (Utilities|Casting|CastToBP_Character Actor)
  (AI|Components|Blackboard|SetValueasBool (AI|GetBlackboard 0) (Utilities|Name|MakeLiteralName "visablePlayer") (.bSuccessfullySensed (Utilities|Struct|BreakAIStimulus Stimulus))))

(event EventBeginPlay
  (bind _returnvalue (AI|GetBlackboard 0))
  (AI|RunBehaviorTree "/Game/Blueprints/AI/AI-tree-test.AI-tree-test")
  (bind _asai_test (Utilities|Casting|CastToAI-TEST (Pawn|GetControlledPawn)))
  (bind _output_get (Variables|Default|SetMyPawn _asai_test))
  (AI|Components|Blackboard|SetValueasBool (AI|GetBlackboard 0) (Utilities|Name|MakeLiteralName "PathLooping") (Variables|/Game/Blueprints/AI/PatrolPath.PatrolPath_C|GetIsLooping (Variables|/Game/Blueprints/AI/AI-TEST.AI-TEST_C|GetPatrolPath _output_get)))
  (Class|BlackboardComponent|SetValueasInt _returnvalue (Utilities|Name|MakeLiteralName "Direction") 1)
  (AI|Components|Blackboard|SetValueasFloat _returnvalue (Utilities|Name|MakeLiteralName "WaitTime") (Variables|/Game/Blueprints/AI/PatrolPath.PatrolPath_C|GetWaitTime (Variables|/Game/Blueprints/AI/AI-TEST.AI-TEST_C|GetPatrolPath (Variables|Default|GetMyPawn)))))

(fn ConstructionScript)